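; BP_HexRoom is a room Blueprint that builds a hex-tiled floor from instanced meshes on FloorHex, sized by Dimensions.
; The construction script clears and rebuilds the floor through CreateHexGrid when the instance count differs from Dimensions X times Y.
; CreateHexGrid places instances via GridToWorld, but its loops overrun Dimensions, so the count exceeds that product and the guard does not prevent rebuilds.
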(fn `CreateHexGrid`
  (bind (_x _y) (break `IntPoint` (`self.Dimensions`)))
  (for _index (range (+ (+ _x 1) 1))
    (for _index_2 (range (+ (+ _y 1) 1))
      (`InstancedStaticMeshComponent.AddInstance` (`self.FloorHex`) (`KismetMathLibrary.Conv_VectorToTransform` (`/Game/Blueprints/BPLib_Hex.GridToWorld` _index _index_2))))))

(fn `UserConstructionScript`
  (bind (_x _y) (break `IntPoint` (`self.Dimensions`)))
  (if (not (== (`InstancedStaticMeshComponent.GetInstanceCount` (`self.FloorHex`)) (* _x _y)))
    (`InstancedStaticMeshComponent.ClearInstances` (`self.FloorHex`))
    (`self.CreateHexGrid`)))