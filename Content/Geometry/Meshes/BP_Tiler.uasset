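; BP_Tiler is a construction-script tool that lays out repeated copies of a mesh as instances.
; It places each instance at MeshSize times its index, leaving gaps at indices in SkipIndexList and extending the range by that list's length.
; Instances are cleared and rebuilt only when their count differs from MeshCount, so size or skip edits alone do not trigger a rebuild.
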(fn `UserConstructionScript`
  (if (!= (`InstancedStaticMeshComponent.GetInstanceCount` (`self.Mesh`)) (`self.MeshCount`))
    (`InstancedStaticMeshComponent.ClearInstances` (`self.Mesh`))
    (for _index (range (+ (+ (- (`self.MeshCount`) 1) (`KismetArrayLibrary.Array_Length` (`self.SkipIndexList`))) 1))
      (if (not (`KismetArrayLibrary.Array_Contains` (`self.SkipIndexList`) _index))
        (`InstancedStaticMeshComponent.AddInstance` (`self.Mesh`) (`KismetMathLibrary.Conv_VectorToTransform` (* (`self.MeshSize`) _index)))))))