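; BP_Alternator is a construction-time tool that lays out a line of alternating instanced meshes.
; When its count check fails (it adds MeshEven's count twice, ignoring MeshOdd), the Construction Script clears and rebuilds MeshEven and MeshOdd.
; Index parity picks the component, and each placement advances CurrentLocation by the opposite parity's size vector.
; SkipIndexList entries extend the loop and break the alternation without leaving gaps.
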(fn `UserConstructionScript`
  (locals (CurrentLocation :type "Vector Structure"))
  (bind _currentlocation (`local.CurrentLocation`))
  (bind _returnvalue (`KismetMathLibrary.Conv_VectorToTransform` _currentlocation))
  (if (!= (+ (`InstancedStaticMeshComponent.GetInstanceCount` (`self.MeshEven`)) (`InstancedStaticMeshComponent.GetInstanceCount` (`self.MeshEven`))) (`self.MeshCount`))
    (`InstancedStaticMeshComponent.ClearInstances` (`self.MeshEven`))
    (`InstancedStaticMeshComponent.ClearInstances` (`self.MeshOdd`))
    (for _index (range (+ (+ (- (`self.MeshCount`) 1) (`KismetArrayLibrary.Array_Length` (`self.SkipIndexList`))) 1))
      (if (`KismetArrayLibrary.Array_Contains` (`self.SkipIndexList`) _index)
        _
        (elif (== (mod _index 2) 0)
          (`InstancedStaticMeshComponent.AddInstance` (`self.MeshEven`) _returnvalue)
          (set `local.CurrentLocation` (+ _currentlocation (`self.OddMeshSize`)))
          (else
            (`InstancedStaticMeshComponent.AddInstance` (`self.MeshOdd`) _returnvalue)
            (set `local.CurrentLocation` (+ _currentlocation (`self.EvenMeshSize`)))))))))