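; BP_Proj is a projectile actor that delivers gameplay ability effects on impact.
; On BeginPlay it generates effect specs from its on-hit effects container using the instigator as source, and makes its collision ignore the instigator while moving.
; On a hit, only the authority adds the hit result to the container, applies it to the struck actor, and destroys the projectile.
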(event `self.ReceiveBeginPlay`
  (bind _returnvalue (`self.GetInstigator`))
  (`GASBlueprintLibrary.GenerateEffectSpecs` (`self.OnHitEffectsContainer`) _returnvalue)
  (`PrimitiveComponent.IgnoreActorWhenMoving` (`self.CollisionComponent`) _returnvalue true))

(event `self.ReceiveHit`
  (params (MyComp :type "PrimitiveComponent Object Reference") (Other :type "Actor Object Reference") (OtherComp :type "PrimitiveComponent Object Reference") (bSelfMoved :type Boolean) (HitLocation :type "Vector Structure") (HitNormal :type "Vector Structure") (NormalImpulse :type "Vector Structure") (Hit :type "HitResult Structure (by ref)"))
  (bind _onhiteffectscontainer (`self.OnHitEffectsContainer`))
  (`/Engine/EditorBlueprintResources/ActorMacros.Switch Has Authority`
    (:`Authority`
      (`GASBlueprintLibrary.AddHitResult` _onhiteffectscontainer Hit)
      (`GASBlueprintLibrary.ApplyEffectApplicationContainerToTarget` _onhiteffectscontainer Other)
      (`self.K2_DestroyActor`))))

(fn `UserConstructionScript`)