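; BP_PlayerPawn is the player's pawn in a turn-driven game, linking the character to its UI.
; On BeginPlay it passes itself to the health bar hosted in its widget component.
; When its turn begins, it creates an action sequencer widget bound to itself, adds it to the viewport and shows the mouse cursor.
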(event `self.ReceiveBeginPlay`
  (bind _aswbp_health_bar (cast `/Game/UI/WBP_HealthBar` (`WidgetComponent.GetUserWidgetObject` (`self.Widget`))))
  (set `/Game/UI/WBP_HealthBar.Character` self _aswbp_health_bar))

(event `OnBeginTurn_1`
  (bind _asplayer_controller (cast `PlayerController` (`self.GetController`)))
  (bind _returnvalue (`|CreateWidget` "/Game/UI/Gloom/Actions/WBP_ActionSequencer.WBP_ActionSequencer_C" _asplayer_controller self))
  (`UserWidget.AddToViewport` _returnvalue 0)
  (set `PlayerController.bShowMouseCursor` true _asplayer_controller))

(fn `UserConstructionScript`)