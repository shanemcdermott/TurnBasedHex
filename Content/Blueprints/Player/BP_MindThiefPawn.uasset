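; BP_MindThiefPawn is the Mind Thief player pawn, which opens the UI for each phase of turn-based play.
; BeginPlay links the health bar on its widget component to the pawn.
; Action selection and turn start events create WBP_ActionSelect and WBP_ActionSequencer respectively, each bound to the pawn, and show the mouse cursor.
; The Enter key calls EndTurn directly.
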(event `self.ReceiveBeginPlay`
  (bind _aswbp_health_bar (cast `/Game/UI/WBP_HealthBar` (`WidgetComponent.GetUserWidgetObject` (`self.Widget_0`))))
  (set `/Game/UI/WBP_HealthBar.Character` self _aswbp_health_bar))

(event `Key|Enter`
  (params (Key :type "Key Structure"))
  (:`Pressed`
    (`self.EndTurn`)))

(event `self.OnBeginActionSelection`
  (bind _asplayer_controller (cast `PlayerController` (`self.GetController`)))
  (bind _returnvalue (`|CreateWidget` "/Game/UI/Gloom/WBP_ActionSelect.WBP_ActionSelect_C" null self))
  (`UserWidget.AddToViewport` _returnvalue 0)
  (set `PlayerController.bShowMouseCursor` true _asplayer_controller))

(event `self.OnBeginTurn`
  (bind _asplayer_controller (cast `PlayerController` (`self.GetController`)))
  (bind _returnvalue (`|CreateWidget` "/Game/UI/Gloom/WBP_ActionSequencer.WBP_ActionSequencer_C" _asplayer_controller self))
  (`UserWidget.AddToViewport` _returnvalue 0)
  (set `PlayerController.bShowMouseCursor` true _asplayer_controller))

(fn `UserConstructionScript`)