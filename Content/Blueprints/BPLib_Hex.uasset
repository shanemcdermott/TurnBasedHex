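; Blueprint function library of hex-grid coordinate helpers, using fixed spacing with odd X columns shifted half a cell in negative Y.
; GridToWorld converts column and row indices into world positions at zero Z.
; SnapToGrid rounds world coordinates per axis before applying the column shift, so results are not always the nearest center, and optionally keeps Z.
; Sqrt3div2 returns the hex ratio constant, though neither function calls it.
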(fn `GridToWorld`
  (params (X :type Integer) (Y :type Integer))
  (returns (WorldLocation :type "Vector Structure"))
  (if (== (mod X 2) 0)
    (return (`KismetMathLibrary.MakeVector` (* X 346.5) (* Y 400.0)))
    (else
      (return (`KismetMathLibrary.MakeVector` (* X 346.5) (- (* Y 400.0) 200.0))))))

(fn `SnapToGrid`
  (params (WorldCoords :type "Vector Structure") (keepZ :type Boolean :default false))
  (returns (GridWorldCoords :type "Vector Structure"))
  (locals (ZVal :type "Float (double-precision)"))
  (bind _returnvalue (`KismetMathLibrary.Round` (/ (.x WorldCoords) 346.5)))
  (bind _returnvalue_2 (`KismetMathLibrary.Round` (/ (.y WorldCoords) 400.0)))
  (if keepZ
    (set `local.ZVal` (.z WorldCoords)))
  (if (== (mod _returnvalue 2) 0)
    (return (`KismetMathLibrary.MakeVector` (* _returnvalue 346.5) (* _returnvalue_2 400.0) (`local.ZVal`)))
    (else
      (return (`KismetMathLibrary.MakeVector` (* _returnvalue 346.5) (- (* _returnvalue_2 400.0) 200.0) (`local.ZVal`))))))

(fn `Sqrt3div2`
  (returns (Result :type "Float (double-precision)"))
  (return 0.866))