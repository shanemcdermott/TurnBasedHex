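; Spawner actor that keeps one instance of its configured class alive at a grid-snapped position.
; The construction script snaps the actor's location to the grid while keeping Z, stores it with the actor's rotation as the spawn transform, and moves an arrow there.
; On Tick, only with authority, it spawns a replacement whenever spawning is enabled and the tracked actor is no longer valid.
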(event `self.ReceiveTick`
  (params (DeltaSeconds :type "Float (single-precision)"))
  (`/Engine/EditorBlueprintResources/ActorMacros.Switch Has Authority`
    (:`Authority`
      (if (`self.SpawningEnabled`)
        (`/Engine/EditorBlueprintResources/StandardMacros.IsValid` (`self.SpawnActor`)
          (:`Is Not Valid`
            (bind _returnvalue (`|SpawnActorFromClass` (`self.SpawnClass`) (`self.SpawnTransform`) "Undefined" "OverrideRootScale" null null))
            (set `self.SpawnActor` _returnvalue)))))))

(fn `UserConstructionScript`
  (bind _outsnappedcoords (`HexagonLib.SnapToGrid` (`self.K2_GetActorLocation`)))
  (set `self.SpawnTransform` (`KismetMathLibrary.MakeTransform` _outsnappedcoords (`self.K2_GetActorRotation`)))
  (`SceneComponent.K2_SetWorldLocation` (`self.Arrow`) _outsnappedcoords false false))