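; BP_GloomGameMode is the game mode for Gloom, choosing which pawn each player spawns with.
; Its GetDefaultPawnClassForController returns the PawnClass stored on BP_PlayerController, falling back to SpectatorPawn for other controllers.
; The event graph holds unconnected authority-only logic that would register a controller in BP_GloomGameState's PConlist and notify the others through OnPlayerJoined, but it never runs.
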(fn `GetDefaultPawnClassForController`
  (params (InController :type "Controller Object Reference"))
  (returns (ReturnValue :type "Object Class Reference"))
  (bind _asbp_player_controller (cast `/Game/Blueprints/Controllers/BP_PlayerController` InController)
    (:`then`
      (return (`GloomPlayerController.PawnClass` _asbp_player_controller)))
    (:`CastFailed`
      (return "/Script/Engine.SpectatorPawn"))))

(fn `UserConstructionScript`)