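; Hex grid tile that tracks the pawn standing on it and shows ally, enemy, selection and highlight states.
; Construction snaps it to the grid and creates a dynamic material for color and opacity.
; Server-only overlap events set or clear the occupant and tint, while UpdateOccupant rescans overlaps and snaps the first pawn to the grid.
; Hover and click are forwarded to the player controller, with separate functions handling selection and highlight visuals.
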(event `self.ReceiveBeginPlay`)

(event `self.ReceiveActorBeginOverlap`
  (params (OtherActor :type "Actor Object Reference"))
  (`/Engine/EditorBlueprintResources/ActorMacros.Switch Has Authority`
    (:`Authority`
      (bind _aspawn (cast `Pawn` OtherActor))
      (`self.SetOccupant` _aspawn)
      (cast `/Game/Blueprints/Player/BP_PlayerPawn` _aspawn
        (:`then`
          (`self.SetColor` (`self.AllyColor`)))
        (:`CastFailed`
          (cast `GloomAICharacter` _aspawn)
          (`self.SetColor` (`self.EnemyColor`)))))))

(event `self.ReceiveActorEndOverlap`
  (params (OtherActor :type "Actor Object Reference"))
  (`/Engine/EditorBlueprintResources/ActorMacros.Switch Has Authority`
    (:`Authority`
      (bind _returnvalue (`self.GetOccupant`))
      (if (== _returnvalue OtherActor)
        (`self.RemoveOccupant`)
        (`self.SetColor` (`self.DefaultColor`))))))

(event `self.ReceiveActorBeginCursorOver`
  (message `/Game/Blueprints/Controllers/BPI_PlayerSelection.SetPlayerHover` (`GameplayStatics.GetPlayerController` 0) self))

(event `self.ReceiveActorOnClicked`
  (params (ButtonPressed :type "Key Structure"))
  (message `/Game/Blueprints/Controllers/BPI_PlayerSelection.SetPlayerSelection` (`GameplayStatics.GetPlayerController` 0) self))

(fn `BeginHighlight`
  (`self.SetOpacity` 0.5))

(fn `EndHighlight`
  (`self.SetOpacity` 0.0))

(fn `OnBeginSelection`
  (locals (SelectedColor :type "LinearColor Structure" :default (struct :`G` 0.133764 :`B` 0.630208 :`A` 1.0)))
  (`self.SetColor` (`local.SelectedColor`)))

(fn `OnEndSelection`
  (`self.SetColor` (`self.DefaultColor`)))

(fn `UpdateOccupant`
  (bind _overlappingactors (`self.GetOverlappingActors` "/Script/Engine.Pawn"))
  (bind _returnvalue (`KismetArrayLibrary.Array_Length` _overlappingactors))
  (bind _output (`|GetArrayItem` _overlappingactors))
  (if (> _returnvalue 0)
    (`KismetSystemLibrary.PrintString` (`KismetStringLibrary.Conv_IntToString` _returnvalue))
    (`self.SetOccupant` _output)
    (`self.K2_SetActorLocation` _output (`HexagonLib.SnapToGrid` (`self.K2_GetActorLocation` _output)) false false)
    (cast `/Game/Blueprints/AI/BP_GloomAICharacter` _output
      (:`then`
        (`self.SetColor` (`self.EnemyColor`)))
      (:`CastFailed`
        (cast `GASCharacter` _output)
        (`self.SetColor` (`self.AllyColor`))))
    (else
      (`KismetSystemLibrary.PrintString` "No Overlaps found")
      (`self.RemoveOccupant`)
      (`self.SetColor` (`self.DefaultColor`)))))

(fn `UserConstructionScript`
  (`self.K2_SetActorLocation` (`HexagonLib.SnapToGrid` (`self.K2_GetActorLocation`)))
  (bind _returnvalue (`PrimitiveComponent.CreateDynamicMaterialInstance` (`self.StaticMesh`) 0 "/Game/Materials/Interface/M_MoveHex.M_MoveHex"))
  (bind _output_get (set `self.NodeMaterial` _returnvalue))
  (bind _returnvalue_2 (`MaterialInstanceDynamic.K2_GetVectorParameterValue` _output_get "Color"))
  (bind _output_get_2 (set `self.DefaultColor` _returnvalue_2))
  (set `self.NodeColor` _output_get_2)
  (`self.SetOpacity` 0.2))