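; BP_Radius is a hex grid actor that displays a ring of neighboring cells around its local origin, apparently as a movement area.
; The construction script creates a dynamic MoveArea material on an instanced static mesh and sets its MaxDistance parameter.
; It then adds one mesh instance at the origin's neighbor in each hex direction.
; An instance-clearing check is left unconnected, and the event graph is empty.
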(fn `UserConstructionScript`
  (bind _returnvalue (`PrimitiveComponent.CreateDynamicMaterialInstance` (`self.InstancedStaticMesh`) 0 "/Game/Materials/Interface/MoveArea.MoveArea"))
  (bind _output_get (set `self.MoveMat` _returnvalue))
  (`MaterialInstanceDynamic.SetScalarParameterValue` _output_get "MaxDistance" 3.0)
  (bind _enumvalue (foreach `EHexDirection`)
    (:`LoopBody`
      (`InstancedStaticMeshComponent.AddInstance` (`self.InstancedStaticMesh`) (`KismetMathLibrary.Conv_VectorToTransform` (`HexagonLib.WorldNeighbor` (`KismetMathLibrary.MakeVector` 0.0) _enumvalue))))))