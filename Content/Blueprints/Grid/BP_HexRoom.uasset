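; BP_HexRoom is a grid room actor that builds a hexagonal floor from its Dimensions in the construction script.
; CreateHexGrid loops over both axes and adds a FloorHex instance at each AxialToWorld position.
; The script clears and rebuilds when the instance count differs from X times Y, though the loop bounds run past Dimensions, so the counts do not line up.
; The event graph holds no active logic.
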(fn `CreateHexGrid`
  (params (Target :type "InstancedStaticMeshComponent Object Reference"))
  (bind (_x _y) (break `IntPoint` (`self.Dimensions`)))
  (for _index (range (+ (+ _x 1) 1))
    (for _index_2 (range (+ (+ _y 1) 1))
      (`InstancedStaticMeshComponent.AddInstance` Target (`KismetMathLibrary.Conv_VectorToTransform` (`HexagonLib.AxialToWorld` _index _index_2))))))

(fn `UserConstructionScript`
  (bind _floorhex (`self.FloorHex`))
  (bind (_x _y) (break `IntPoint` (`self.Dimensions`)))
  (if (not (== (`InstancedStaticMeshComponent.GetInstanceCount` (`self.FloorHex`)) (* _x _y)))
    (`InstancedStaticMeshComponent.ClearInstances` _floorhex)
    (`self.CreateHexGrid` _floorhex)))