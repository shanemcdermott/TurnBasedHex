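; BP_PlayerController is a player controller that tracks the player's hovered and selected grid nodes and drives a cursor actor.
; It spawns BP_PlayerCursor on BeginPlay and snaps it to the hovered node's grid position, exposing hover, selection and cursor location through getters.
; Selection changes notify the old and new nodes, then set the new node's occupant as the Gloom pawn's target.
; ServerConfirmReadyToStartRound flags the player as ready for the round.
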(event `self.ReceiveBeginPlay`
  (bind _returnvalue (`|SpawnActorFromClass` "/Game/Blueprints/Controllers/BP_PlayerCursor.BP_PlayerCursor_C" (`KismetMathLibrary.Conv_VectorToTransform` (0.0 0.0 0.0)) "AlwaysSpawn" "OverrideRootScale" null null))
  (set `self.CursorPtr` _returnvalue))

(event `/Game/Blueprints/Controllers/BPI_PlayerSelection.SetPlayerSelection`
  (params (CurrentSelection :type "/Game/Blueprints/Grid/BP_HexNode Object Reference"))
  (bind _selectednode (`self.SelectedNode`))
  (`/Engine/EditorBlueprintResources/StandardMacros.IsValid` _selectednode
    (:`Is Valid`
      (`/Game/Blueprints/Grid/BP_HexNode.OnEndSelection` _selectednode))
    (:`Is Not Valid`
      _))
  (bind _output_get (set `self.SelectedNode` CurrentSelection))
  (`/Game/Blueprints/Grid/BP_HexNode.OnBeginSelection` _output_get)
  (bind _returnvalue (`GameNode.GetOccupant` _output_get))
  (`GASCharacter.SetTarget` (`self.GetGloomPawn`) _returnvalue))

(event `/Game/Blueprints/Controllers/BPI_PlayerSelection.SetPlayerHover`
  (params (HoverNode :type "/Game/Blueprints/Grid/BP_HexNode Object Reference"))
  (bind _output_get (set `self.HoveredNode` HoverNode))
  (`/Engine/EditorBlueprintResources/StandardMacros.IsValid` _output_get
    (:`Is Valid`
      (`self.K2_SetActorLocation` (`self.CursorPtr`) (`HexagonLib.SnapToGrid` (`self.K2_GetActorLocation` _output_get)) false false))))

(event `ServerConfirmReadyToStartRound`
  (set `self.bIsReadyToStartRound` true))

(fn `GetCurrentHover`
  (returns (HoveredNode :type "/Game/Blueprints/Grid/BP_HexNode Object Reference"))
  (return (`self.HoveredNode`)))

(fn `GetCurrentSelection`
  (returns (CurrentSelection :type "/Game/Blueprints/Grid/BP_HexNode Object Reference"))
  (return (`self.SelectedNode`)))

(fn `GetCursorLocation`
  (returns (CurrentLocation :type "Vector Structure"))
  (bind _cursorptr (`self.CursorPtr`))
  (`/Engine/EditorBlueprintResources/StandardMacros.IsValid` _cursorptr
    (:`Is Valid`
      (return (`self.K2_GetActorLocation` _cursorptr)))
    (:`Is Not Valid`
      (return (0.0 0.0 0.0)))))

(fn `UserConstructionScript`)